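; BP_MasterItem is a world item pickup that carries MasterItem data and can be collected into a player's inventory.
; On BeginPlay, a text render shows the item's name and stack size.
; InventoryInteract casts the interacting player's controller to MyPlayerController and passes the item ID and stack size to AddItem with that controller's InventoryActor.
; The pickup then destroys itself without checking whether the add succeeded.
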(event EventBeginPlay
  (bind _masteritem (Variables|Default|GetMasterItem))
  (bind (_itemname _stacksize) (Utilities|Struct|BreakMasterItemStruct _masteritem))
  (Rendering|Components|TextRender|SetText (Variables|Default|GetTextRender) (Utilities|Text|ToText(String) (Utilities|String|Append _itemname "/" (Utilities|String|ToString(Integer) _stacksize)))))

(event EventInventoryInteract
  (params (MyPlayer :type My%20Player%20Object%20Reference))
  (bind _masteritem (Variables|Default|GetMasterItem))
  (bind (_itemid _stacksize) (Utilities|Struct|BreakMasterItemStruct _masteritem))
  (bind _asmy_player_controller (Utilities|Casting|CastToMyPlayerController (Pawn|GetController MyPlayer)))
  (CallFunction|AddItem _itemid _stacksize (Variables|/Game/Player/MyPlayerController.MyPlayerController_C|GetInventoryActor _asmy_player_controller))
  (Actor|DestroyActor))

(fn ConstructionScript)