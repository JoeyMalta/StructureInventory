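; BP_WorkBench is an interactable workbench that gives players access to a crafting-style inventory.
; On BeginPlay, the authority spawns and stores a owned 3x3 inventory actor that uses the GameWorkBench widget.
; An inventory interaction forwards to a server event, which validates the player and has its MyPlayerController open the bench's storage alongside the inventory.
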(event Custom|SRV_Interact
  (params (MyPlayer :type My%20Player%20Object%20Reference))
  (Utilities|IsValid MyPlayer
    (:Is%20Valid
      (bind _asmy_player_controller (Utilities|Casting|CastToMyPlayerController (Pawn|GetController MyPlayer)))
      (Default|OpenStorage _asmy_player_controller (Variables|Default|GetInventoryActor))
      (Default|OpenInventory _asmy_player_controller))))

(event EventBeginPlay
  (Networking|SwitchHasAuthority
    (:Authority
      (bind _returnvalue (Game|SpawnActorfromClass "/Game/Inventory/InventoryActor.InventoryActor_C" (Transformation|GetActorTransform) "AlwaysSpawn" self 3 3 12 false "/Game/Crafting/GameWorkBench.GameWorkBench_C" 0))
      (Variables|Default|SetInventoryActor _returnvalue))))

(event EventInventoryInteract
  (params (MyPlayer :type My%20Player%20Object%20Reference))
  (CallFunction|SRVInteract MyPlayer))

(fn ConstructionScript)