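; BP_MasterItem is a world item pickup, showing the mesh and stack size text from its MasterItem data on BeginPlay.
; Interact calls SRV_AddItems, which adds the item and quantity to the interacting player's InventoryComponent on their PlayerState, then destroys the actor.
; Mesh hits call SRV_PlaySound to play a sound at the item's location; the SRV prefix suggests both events run on the server.
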(event OnComponentHit(MasterItemStaticMesh)
  (params (HitComponent :type Primitive%20Component%20Object%20Reference) (OtherActor :type Actor%20Object%20Reference) (OtherComp :type Primitive%20Component%20Object%20Reference) (NormalImpulse :type Vector :default "0, 0, 0") (Hit :type Hit%20Result%20Structure%20%28by%20ref%29))
  (CallFunction|SRVPlaySound))

(event Custom|SRV_PlaySound
  (Audio|PlaySoundatLocation 0 (Transformation|GetActorLocation) "0, 0, 0" 1.0 1.0 0.0 0 0 0))

(event Custom|SRV_AddItems
  (params (NewParam :type My%20Player%20Object%20Reference))
  (bind (_masteritem _quantity) (Utilities|GetMasterItem))
  (Default|AddItem (Variables|/Game/MyPlayer/MyPlayerState.MyPlayerState_C|GetInventoryComponent (Variables|/Game/MyPlayer/MyPlayer.MyPlayer_C|GetMyPlayerState NewParam)) _masteritem _quantity)
  (Actor|DestroyActor))

(event EventInteract
  (params (MyPlayer :type My%20Player%20Object%20Reference))
  (CallFunction|SRVAddItems MyPlayer))

(event EventBeginPlay
  (Components|StaticMesh|SetStaticMesh (Variables|Default|GetMasterItemStaticMesh) (Utilities|Struct|BreakMasterItemStruct (Variables|Default|GetMasterItem)))
  (Rendering|Components|TextRender|SetText (Variables|Default|GetTextRender) (Utilities|Text|ToText(Integer) (Utilities|Struct|BreakMasterItemStruct (Variables|Default|GetMasterItem)))))

(fn ConstructionScript)